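; Enemy AI character that chases the player and plays an attack montage once its PawnSensing component sees a pawn.
; Sighting sets IsSeenPlayer, calls FollowPlayer to enable and trigger an attack, then runs AIMoveTo toward player 0.
; The attack branch also fires from the move's immediate and success outputs, with CanAttack gating it for the montage's duration.
; Tick halts active movement until IsSeenPlayer is set, and nothing here clears that flag.
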(event `self.ReceiveTick`
  (params (DeltaSeconds :type "Float (single-precision)"))
  (bind _output_get (set `self.IsSeenPlayer` (`self.IsSeenPlayer`)))
  (if (not _output_get)
    (`NavMovementComponent.StopActiveMovement` (`self.CharacterMovement`))))

(event `self.PawnSensing.OnSeePawn`
  (params (Pawn :type "Pawn Object Reference"))
  (set `self.IsSeenPlayer` true)
  (`self.FollowPlayer`)
  (if (`self.IsSeenPlayer`)
    (`|AIMoveTo` self (0.0 0.0 0.0) (`GameplayStatics.GetPlayerCharacter` 0) 75.0 (`self.CanAttack`)
      (:`then`
        _)
      (:`OnSuccess`
        _))
    (if (`self.CanAttack`) :!label _label
      (set `self.CanAttack` false)
      (bind _returnvalue (`self.PlayAnimMontage` null))
      (`KismetSystemLibrary.Delay` _returnvalue)
      (set `self.CanAttack` (stale _output_get))
      (else
        (bind _output_get (set `self.IsSeenPlayer` true))))))

(event `FollowPlayer`
  (set `self.CanAttack` true)
  (goto _label))

(fn `UserConstructionScript`)